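; Player character that moves through Enhanced Input and drills overlapping BPI_Damage actors, spending a rechargeable drill gauge shown on WB_UI.
; Drilling sends damage from DrillZone overlaps and sets GettingDrilled, which blocks movement, spawns effects and changes GameInstance Speed.
; G triggers a timeline super drill with boosted damage and ramped Speed.
; Tick jiggles the movement component and runs recharge and drill-state checks; death only prints, and deflect logic is unwired.
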(event `self.ReceiveBeginPlay`
  ;[0.1216 0.1216 0.1216] BeginPlay
  (`|ExecutionSequence`
    (:`then_0`
      (bind _asplayer_controller (cast `PlayerController` (`self.GetController`)))
      (bind _returnvalue (pcsubsystem `EnhancedInputLocalPlayerSubsystem` _asplayer_controller))
      (`/Engine/EditorBlueprintResources/StandardMacros.IsValid` _returnvalue
        (:`Is Valid`
          (`EnhancedInputSubsystemInterface.AddMappingContext` _returnvalue "/Game/Core/Input/IMC_MyInput.IMC_MyInput" 0 (struct)))))
    (:`then_1`
      (bind _output_get (set `self.MaxHealth` 5.0))
      (set `self.CurrentHealth` _output_get))
    (:`then_2`
      (bind _returnvalue_2 (`|CreateWidget` "/Game/Core/Assets/UI/Character/WB_UI.WB_UI_C"))
      (bind _output_get_2 (set `self.WB_main` _returnvalue_2))
      (`UserWidget.AddToViewport` _output_get_2 0))))

(event `EnhancedInput|/Game/Core/Input/Actions/MyMove`
  (params (ActionValue :type "Vector2D Structure") (ElapsedSeconds :type "Float (double-precision)") (TriggeredSeconds :type "Float (double-precision)") (InputAction :type "InputAction Object Reference" :default "/Game/Core/Input/Actions/MyMove.MyMove"))
  ;[0.1216 0.1216 0.1216] Movement
  (:`Triggered`
    (if (not (`self.gettingDrilled`))
      (`self.AddMovementInput` (`self.GetActorForwardVector`) ActionValue_X)
      (`self.AddMovementInput` (`self.GetActorRightVector`) ActionValue_Y))))

(event `InterfaceSent`
  (bind _overlappingactors (`PrimitiveComponent.GetOverlappingActors` (`self.DrillZone`) null))
  ;[0.06667 0.06667 0.06667] Interface
  (bind _candrill (`self.CanDrill`))
  (if _candrill
    (if (!= (`KismetArrayLibrary.Array_Length` _overlappingactors) 0)
      (for _array_element _overlappingactors
        (if (`KismetSystemLibrary.DoesImplementInterface` _array_element "/Game/Core/Assets/Blueprints/BPI_Damage.BPI_Damage_C")
          (message `/Game/Core/Assets/Blueprints/BPI_Damage.BPI_Damage` _array_element (`self.Damage`))
          (set `self.gettingDrilled` true)))
      (else
        (set `self.gettingDrilled` false)))))

(event `self.ReceiveTick`
  (params (DeltaSeconds :type "Float (single-precision)"))
  (`|ExecutionSequence`
    (:`then_0`
      (`self.UpdateMovement`))
    (:`then_1`
      (if (and (not (`self.isDrilling`)) (< (`self.drillGauge`) 100.0))
        (if (< (`self.DrillGauge`) 10.0)
          (set `self.WaitForCharge` true)
          (else
            (set `self.WaitForCharge` false)))
        (`KismetSystemLibrary.Delay` 0.1)
        (bind _output_get (set `self.drillGauge` (+ 1.0 (`self.DrillGauge`))))
        (`KismetSystemLibrary.PrintString` (`KismetStringLibrary.Conv_DoubleToString` _output_get) true false (struct :`G` 1.0 :`B` 0.028727 :`A` 1.0) 120.0 "DrillGauge")))
    (:`then_2`
      (if (`self.isSuperDrilling`)
        (`self.InterfaceSent`)))
    (:`then_3`
      (if (`self.gettingDrilled`)
        (`|ExecutionSequence`
          (:`then_0`
            (`NiagaraFunctionLibrary.SpawnSystemAtLocation` "/Game/Core/Assets/VFX/DrillEmitter.DrillEmitter" (`self.K2_GetActorLocation`) (struct) (3.0 3.0 3.0))
            (`/Engine/EditorBlueprintResources/StandardMacros.Do N` 1 :!label _label
              (:`Exit`
                (bind _gameinstance (`/Game/Core/Assets/Blueprints/BPL_Library.CastToGameInstance`))
                (set `/Game/Core/Assets/Blueprints/BP_GameInstance.Speed` 0.0 _gameinstance))))
          (:`then_1`
            (goto _label_2 :!via `Reset`)))
        (else
          (`|ExecutionSequence`
            (:`then_0`
              (`/Engine/EditorBlueprintResources/StandardMacros.Do N` 1 :!label _label_2
                (:`Exit`
                  (bind _gameinstance_2 (`/Game/Core/Assets/Blueprints/BPL_Library.CastToGameInstance`))
                  (set `/Game/Core/Assets/Blueprints/BP_GameInstance.Speed` 10000.0 _gameinstance_2))))
            (:`then_1`
              (goto _label :!via `Reset`))))))))

(event `/Game/Core/Assets/Blueprints/BPI_Damage.BPI_Damage`
  (params (Damage :type Integer))
  (bind _output_get (set `self.CurrentHealth` (- (`self.CurrentHealth`) Damage)))
  (`KismetSystemLibrary.PrintString` (`KismetStringLibrary.Conv_DoubleToString` _output_get))
  (if (<= (`self.CurrentHealth`) 0.0)
    (`KismetSystemLibrary.PrintString` "DEAAAAAAAAAAAAAAAAAAAAAAAAAAD" true true (struct :`R` 1.0 :`G` 0.0169 :`A` 1.0))))

(event `EnhancedInput|/Game/Core/Input/Actions/MyDrill`
  (params (ActionValue :type Boolean) (ElapsedSeconds :type "Float (double-precision)") (TriggeredSeconds :type "Float (double-precision)") (InputAction :type "InputAction Object Reference" :default "/Game/Core/Input/Actions/MyDrill.MyDrill"))
  (:`Triggered`
    (`self.InterfaceSent`)))

(event `EnhancedInput|/Game/Core/Input/Actions/MyDrill`
  (params (ActionValue :type Boolean) (ElapsedSeconds :type "Float (double-precision)") (TriggeredSeconds :type "Float (double-precision)") (InputAction :type "InputAction Object Reference" :default "/Game/Core/Input/Actions/MyDrill.MyDrill"))
  (:`Triggered`
    (bind _candrill (`self.CanDrill`))
    (if _candrill
      (set `self.isDrilling` true)
      (`KismetSystemLibrary.Delay` 0.05)
      (`KismetSystemLibrary.PrintString` (`KismetStringLibrary.Conv_DoubleToString` (`self.drillGauge`)) true false (struct :`G` 1.0 :`B` 0.032499 :`A` 1.0) 120.0 "DrillGauge")
      (set `self.drillGauge` (- (`self.DrillGauge`) 1.0))
      (`/Game/Core/Assets/UI/Character/WB_UI.set_drill_gauge` (`self.WB_main`))
      (else
        (set `self.isDrilling` false :!label _label_3)
        (set `self.gettingDrilled` false))))
  (:`Completed`
    (goto _label_3)))

(event `Key|G`
  (params (Key :type "Key Structure"))
  (:`Pressed`
    (bind _candrill (`self.CanDrill`))
    (if _candrill
      (set `self.isSuperDrilling` true)
      (set `self.Damage` 1000)
      (bind (_direction _alpha) (`Timeline|Timeline` :!via `PlayFromStart`)
        (:`Update`
          (`self.InterfaceSent`)
          (bind _gameinstance (`/Game/Core/Assets/Blueprints/BPL_Library.CastToGameInstance`))
          (set `/Game/Core/Assets/Blueprints/BP_GameInstance.Speed` (`KismetMathLibrary.Lerp` 10000.0 50000.0 _alpha) _gameinstance))
        (:`Finished`
          (set `self.Damage` 3)
          (set `self.isSuperDrilling` false))))))

(fn `CanDrill`
  (returns (CanDrill :type Boolean))
  (return (and (> (`self.DrillGauge`) 0.0) (not (`self.WaitForCharge`)))))

(fn `UpdateMovement`
  (bind _returnvalue (`self.K2_GetActorRotation`))
  (bind _charactermovement (`self.CharacterMovement`))
  (`MovementComponent.K2_MoveUpdatedComponent` _charactermovement (0.0 0.1 0.0) _returnvalue true false)
  (`MovementComponent.K2_MoveUpdatedComponent` _charactermovement (0.0 -0.1 0.0) _returnvalue true false))

(fn `UserConstructionScript`)