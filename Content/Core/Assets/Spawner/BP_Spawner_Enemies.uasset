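; Enemy spawner that continually spawns BP_Cygnus actors at random points marked by thirteen arrow components.
; Tick uses an IsSpawning flag to gate a randomly delayed cycle that picks an arrow location, then calls Spawn.
; Spawn waits briefly, creates the actor with collision adjustment, and clears the flag.
; An SPeed function, uncalled here, steps the spawner along negative X from a given actor's location, wrapping at a limit.
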(event `self.ReceiveTick`
  (params (DeltaSeconds :type "Float (single-precision)"))
  (if (not (`self.isSpawning`))
    (set `self.isSpawning` true)
    (`KismetSystemLibrary.Delay` (`KismetMathLibrary.RandomFloatInRange` 1.0 1.5))
    (set `self.SpawnPoint` (`SceneComponent.K2_GetComponentLocation` (`|GetArrayItem` (`|MakeArray` (`self.Arrow`) (`self.Arrow1`) (`self.Arrow2`) (`self.Arrow3`) (`self.Arrow4`) (`self.Arrow5`) (`self.Arrow6`) (`self.Arrow7`) (`self.Arrow8`) (`self.Arrow9`) (`self.Arrow10`) (`self.Arrow11`) (`self.Arrow12`)) (`KismetMathLibrary.RandomIntegerInRange` 0 12))))
    (`self.Spawn`)))

(event `Spawn`
  (`KismetSystemLibrary.Delay` 0.43)
  (`|SpawnActorFromClass` "/Game/Core/Enemy/BP_Cygnus.BP_Cygnus_C" (`KismetMathLibrary.MakeTransform` (`self.SpawnPoint`)) "AdjustIfPossibleButAlwaysSpawn" "OverrideRootScale" null null)
  (set `self.isSpawning` false))

(fn `NewFunction`)

(fn `SPeed`
  (params (actor :type "Actor Object Reference"))
  (bind (_returnvalue_x _returnvalue_y _returnvalue_z) (`KismetMathLibrary.BreakVector` (`self.K2_GetActorLocation` actor)))
  (bind _returnvalue (+ _returnvalue_x -100.0))
  (if (<= _returnvalue -10000.0)
    (`self.K2_SetActorLocation` (89660.0 0.0 -140.5))
    (else
      (`self.K2_SetActorLocation` (`KismetMathLibrary.MakeVector` _returnvalue _returnvalue_y _returnvalue_z)))))

(fn `UserConstructionScript`)