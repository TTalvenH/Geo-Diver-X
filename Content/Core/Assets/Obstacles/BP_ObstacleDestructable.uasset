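; BP_ObstacleDestructable is a destructible cube obstacle that travels along negative X and destroys itself past a fixed limit.
; Tick calls Speed, which applies a fixed, frame-rate-dependent step without sweep.
; Each cube hit lowers and prints Health; at zero, the cube loses visibility and collision, then reactivates with full Health after a delay.
; Cube component activation also triggers the same reactivation.
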(event `self.ReceiveTick`
  (params (DeltaSeconds :type "Float (single-precision)"))
  (`self.Speed` self))

(event `self.Cube.OnComponentActivated`
  (params (Component :type "ActorComponent Object Reference") (bReset :type Boolean))
  (`self.ReactivateObstacle`))

(event `DecrementHealth`
  (set `self.Health` (- (`self.Health`) 10)))

(event `HideObstacle`
  (`SceneComponent.ToggleVisibility` (`self.Cube`) false)
  (`PrimitiveComponent.SetCollisionEnabled` (`self.Cube`) "NoCollision")
  (`KismetSystemLibrary.Delay` 5.0)
  (`self.ReactivateObstacle`))

(event `ReactivateObstacle`
  (set `self.Health` 100)
  (`PrimitiveComponent.SetCollisionEnabled` (`self.Cube`) "QueryAndPhysics")
  (`SceneComponent.SetVisibility` (`self.Cube`) true false))

(event `self.Cube.OnComponentHit`
  (params (HitComponent :type "PrimitiveComponent Object Reference") (OtherActor :type "Actor Object Reference") (OtherComp :type "PrimitiveComponent Object Reference") (NormalImpulse :type "Vector Structure") (Hit :type "HitResult Structure (by ref)"))
  (`self.DecrementHealth`)
  (`KismetSystemLibrary.PrintString` (`KismetStringLibrary.Conv_IntToString` (`self.Health`)))
  (if (<= (`self.Health`) 0)
    (`self.HideObstacle`)))

(fn `Speed`
  (params (Actor :type "Actor Object Reference"))
  (bind (_returnvalue_x _returnvalue_y _returnvalue_z) (`KismetMathLibrary.BreakVector` (`self.K2_GetActorLocation` Actor)))
  (bind _returnvalue (+ _returnvalue_x -100.0))
  (if (<= _returnvalue -10000.0)
    (`self.K2_DestroyActor`)
    (else
      (`self.K2_SetActorLocation` (`KismetMathLibrary.MakeVector` _returnvalue _returnvalue_y _returnvalue_z)))))

(fn `UserConstructionScript`)