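; BP_TRASH is an enemy projectile that deals damage on contact.
; On BeginPlay it homes on the player's capsule, then turns homing off after a short delay so it flies on unguided.
; Each Tick it prints overlapping actors, sends BPI_Damage to any that implement it and destroys itself.
; An unconnected branch holds manual movement and deflection by a drilling player, so that logic never runs.
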(event `self.ReceiveBeginPlay`
  (`|ExecutionSequence`
    (:`then_0`
      (set `self.xTimes` 1.0)
      (set `self.isDeflected` false))
    (:`then_1`
      (set `ProjectileMovementComponent.HomingTargetComponent` (`Character.CapsuleComponent` (`GameplayStatics.GetPlayerCharacter` 0)) (`self.ProjectileMovement`))
      (`KismetSystemLibrary.Delay` 0.2)
      (set `ProjectileMovementComponent.bIsHomingProjectile` false (`self.ProjectileMovement`)))))

(event `self.ReceiveTick`
  (params (DeltaSeconds :type "Float (single-precision)"))
  (for _array_element (`self.GetOverlappingActors` null)
    (`KismetSystemLibrary.PrintString` (`KismetSystemLibrary.GetDisplayName` _array_element))
    (if (`KismetSystemLibrary.DoesImplementInterface` _array_element "/Game/Core/Assets/Blueprints/BPI_Damage.BPI_Damage_C")
      (message `/Game/Core/Assets/Blueprints/BPI_Damage.BPI_Damage` _array_element 1)
      (`self.K2_DestroyActor`))))

(fn `UserConstructionScript`)