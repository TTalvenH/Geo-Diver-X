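; Enemy projectile that aims at the player, deals damage on overlap and can be deflected back at BP_Cygnus.
; On spawn it targets the player's capsule, switches homing off shortly after, then enables WorldDynamic overlaps after a brief delay.
; Tick polls overlaps for BPI_Damage actors: if the player is deflecting, it homes on its Cygnus owner or self-destructs without an owner.
; Otherwise it damages the actor and destroys itself.
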(event `self.ReceiveBeginPlay`
  (`|ExecutionSequence`
    (:`then_0`
      (set `self.xTimes` 1.0)
      (set `self.isDeflected` false))
    (:`then_1`
      (set `ProjectileMovementComponent.HomingTargetComponent` (`Character.CapsuleComponent` (`GameplayStatics.GetPlayerCharacter` 0)) (`self.ProjectileMovement`))
      (`KismetSystemLibrary.Delay` 0.1)
      (set `ProjectileMovementComponent.bIsHomingProjectile` false (`self.ProjectileMovement`)))
    (:`then_2`
      (`KismetSystemLibrary.Delay` 0.2)
      (`PrimitiveComponent.SetCollisionResponseToChannel` (`self.Sphere`) "ECC_WorldDynamic" "ECR_Overlap"))))

(event `self.ReceiveTick`
  (params (DeltaSeconds :type "Float (single-precision)"))
  (bind _returnvalue (`self.GetOwner`))
  (for _array_element (`self.GetOverlappingActors` null)
    (if (`KismetSystemLibrary.DoesImplementInterface` _array_element "/Game/Core/Assets/Blueprints/BPI_Damage.BPI_Damage_C")
      (bind _asbp_my_2dcharacter (cast `/Game/Core/Character/BP_My2DCharacter` (`GameplayStatics.GetPlayerCharacter` 0)))
      (if (`/Game/Core/Character/BP_My2DCharacter.isDeflecting` _asbp_my_2dcharacter)
        (set `ProjectileMovementComponent.bIsHomingProjectile` true (`self.ProjectileMovement`))
        (`/Engine/EditorBlueprintResources/StandardMacros.IsValid` _returnvalue
          (:`Is Valid`
            (bind _asbp_cygnus (cast `/Game/Core/Enemy/BP_Cygnus` _returnvalue))
            (set `ProjectileMovementComponent.HomingTargetComponent` (`/Game/Core/Enemy/BP_Cygnus.StaticMesh` _asbp_cygnus) (`self.ProjectileMovement`)))
          (:`Is Not Valid`
            (`self.K2_DestroyActor`)))
        (else
          (message `/Game/Core/Assets/Blueprints/BPI_Damage.BPI_Damage` _array_element 1)
          (`self.K2_DestroyActor`))))))

(fn `UserConstructionScript`)