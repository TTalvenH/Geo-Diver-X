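; BP_Cygnus is an enemy actor with debug firing and a damage-and-death response.
; It enables player input on BeginPlay so the K key spawns a BP_Projectile offset along world X from its location, a stand-in for automatic firing.
; The BPIDamage event destroys it when a single hit's damage reaches Health, otherwise printing Health, which never drops because the subtraction uses zero instead of Damage.
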(event `self.ReceiveBeginPlay`
  ;[1 1 1] Comment
  ;;[1 1 1] Needs to happen by itself, not from button press. DEBUG
  (`self.EnableInput` (`GameplayStatics.GetPlayerController` 0)))

(event `Key|K`
  (params (Key :type "Key Structure"))
  (bind _returnvalue (`self.GetTransform`))
  ;[1 1 1] Comment
  (:`Pressed`
    (`|SpawnActorFromClass` "/Game/Core/Enemy/BP_Projectile.BP_Projectile_C" (`KismetMathLibrary.MakeTransform` (`KismetMathLibrary.MakeVector` (+ (.x (.location _returnvalue)) 200.0) (.y (.location _returnvalue)) (.z (.location _returnvalue)))) "Undefined" "OverrideRootScale" null null)))

(event `/Game/Core/Assets/Blueprints/BPI_Damage.BPI_Damage`
  (params (Damage :type Integer))
  (bind _health (`self.Health`))
  ;[1 1 1] Take Damage and Die event
  (set `self.Health` (- _health 0.0))
  (if (<= _health Damage)
    (`KismetSystemLibrary.PrintString` "Enemy Died")
    (`self.K2_DestroyActor`)
    (else
      (`KismetSystemLibrary.PrintString` "Boom")
      (`KismetSystemLibrary.PrintString` (`KismetStringLibrary.Conv_DoubleToString` (`self.Health`))))))

(fn `UserConstructionScript`)