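; BP_ScrollingField is a scrolling level actor that moves two referenced actors along negative X in a repeating loop.
; Each Tick passes both to Speed, which steps them a fixed, frame-rate-dependent distance and snaps them to the world origin at the X limit.
; Tick also prints a debug string, and a BP_Shape spawn node is left unconnected.
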(event `self.ReceiveBeginPlay`)

(event `self.ReceiveTick`
  (params (DeltaSeconds :type "Float (single-precision)"))
  (`KismetSystemLibrary.PrintString` "Hello")
  (`self.Speed` (`self.Actor2`))
  (`self.Speed` (`self.Atcor`)))

(fn `Speed`
  (params (Actor :type "Actor Object Reference"))
  (bind (_returnvalue_x _returnvalue_y _returnvalue_z) (`KismetMathLibrary.BreakVector` (`self.K2_GetActorLocation` Actor)))
  (bind _returnvalue (+ _returnvalue_x -10.0))
  (if (<= _returnvalue -1000.0)
    (`self.K2_SetActorLocation` Actor (0.0 0.0 0.0) false false)
    (else
      (`self.K2_SetActorLocation` Actor (`KismetMathLibrary.MakeVector` _returnvalue _returnvalue_y _returnvalue_z) false false))))

(fn `UserConstructionScript`)